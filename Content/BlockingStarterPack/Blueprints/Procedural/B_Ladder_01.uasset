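; B_Ladder_01 is a procedural ladder Blueprint from the blocking starter pack, built on an instanced static mesh.
; Its construction script runs the parent's script, then applies HorizontalMat to material slot 0 and VerticalMat to slot 1, skipping either if unset.
; The file adds no instance placement or runtime logic of its own, and its event stubs are disabled.
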(event EventBeginPlay
  (|CallParentFunction) ; This node is disabled and will not be called.\nDrag off pins to build functionality.
)

(event Collision|EventActorBeginOverlap
  (params (OtherActor :type Actor%20Object%20Reference))
  (|CallParentFunction OtherActor) ; This node is disabled and will not be called.\nDrag off pins to build functionality.
)

(event EventTick
  (params (DeltaSeconds :type Float%20%28single-precision%29))
  (|CallParentFunction DeltaSeconds) ; This node is disabled and will not be called.\nDrag off pins to build functionality.
)

(fn ConstructionScript
  (bind _vertical_mat (Variables|Default|GetVertical%20Mat))
  (bind _horizontal_mat (Variables|Default|GetHorizontal%20Mat))
  (|CallParentFunction)
  (Utilities|FlowControl|Sequence
    (:then_0
      (Utilities|IsValid _horizontal_mat
        (:Is%20Valid
          (Rendering|Material|SetMaterial (Variables|Default|GetInstancedStaticMesh) 0 _horizontal_mat))))
    (:then_1
      (Utilities|IsValid _vertical_mat
        (:Is%20Valid
          (Rendering|Material|SetMaterial (Variables|Default|GetInstancedStaticMesh) 1 _vertical_mat))))))