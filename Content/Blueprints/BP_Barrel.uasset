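; BP_Barrel is a storage barrel that opens when the first-person character enters its sphere and closes when they leave.
; A timeline played forward or in reverse rotates the hinge to swing it open or shut.
; The chest menu widget is created at BeginPlay with the inventory component, then added to the viewport once opening finishes, alongside debug text naming the first item.
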(event OnComponentBeginOverlap(Sphere)
  (params (OverlappedComponent :type Primitive%20Component%20Object%20Reference) (OtherActor :type Actor%20Object%20Reference) (OtherComp :type Primitive%20Component%20Object%20Reference) (OtherBodyIndex :type Integer) (bFromSweep :type Boolean) (SweepResult :type Hit%20Result%20Structure%20%28by%20ref%29))
  (Utilities|Casting|CastToBP_FirstPersonCharacter OtherActor)
  (CallFunction|OpenBarrel false))

(event OnComponentEndOverlap(Sphere)
  (params (OverlappedComponent :type Primitive%20Component%20Object%20Reference) (OtherActor :type Actor%20Object%20Reference) (OtherComp :type Primitive%20Component%20Object%20Reference) (OtherBodyIndex :type Integer))
  (Utilities|Casting|CastToBP_FirstPersonCharacter OtherActor)
  (CallFunction|OpenBarrel true))

(event Custom|open%20barrel
  (params (Reverse :type Boolean))
  (if Reverse
    (bind _newtrack_0 (Timeline|Open%20Timeline Reverse)
      (:Update
        (Transformation|SetRelativeRotation (Variables|Default|Gethinge) (Math|Rotator|MakeRotator (Math|Float|Lerp 0.0 -6e+01 _newtrack_0) 0.0 0.0) false false))
      (:Finished
        (if (not Reverse)
          (Development|PrintText "Opening Barrel")
          (UserInterface|Viewport|AddtoViewport (Variables|Default|GetChestMenu) 0)
          (Development|PrintText (Utilities|Text|FormatText "First item in barrel is a {name}." (.Name (Utilities|Struct|BreakS_Item (Utilities|Array|Get(acopy) (Variables|Default|GetInventory))))) true true "(R=0.000000,G=0.660000,B=1.000000,A=1.000000)" 2e+01))))
    (else
      (Timeline|Open%20Timeline Play))))

(event EventBeginPlay
  (bind _returnvalue (UserInterface|CreateWidget "/Game/Widgets/W_ChestMenuu.W_ChestMenuu_C" 0 (Variables|Default|GetBPC_Inventory))) ; create it now, show it later
  (Variables|Default|SetChestMenu _returnvalue))

(fn ConstructionScript)