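; BP_Spawner is a spawner actor that repeatedly spawns a configurable class at its SpawnLocation.
; A self-recalling event starts one second after BeginPlay and retries every five seconds, skipping spawns that would collide.
; When Looping is off, a first-person character overlapping the Trigger registers an actor with GM_SaveLoad's LevelState.
; The Activate event destroys the spawner, while the spawn loop itself never checks Looping.
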(event OnComponentBeginOverlap(Trigger)
  (params (OverlappedComponent :type Primitive%20Component%20Object%20Reference) (OtherActor :type Actor%20Object%20Reference) (OtherComp :type Primitive%20Component%20Object%20Reference) (OtherBodyIndex :type Integer) (bFromSweep :type Boolean) (SweepResult :type Hit%20Result%20Structure%20%28by%20ref%29))
  (if (not (Variables|Default|GetLooping)) ; if we are looping, don't do anything
    (Utilities|Casting|CastToBP_FirstPersonCharacter OtherActor)
    (bind _asgm_save_load (Utilities|Casting|CastToGM_SaveLoad (Game|GetGameMode)))
    (Default|AddActor (Variables|/Game/Blueprints/SavingLoading/GM_SaveLoad.GM_SaveLoad_C|GetLevelState _asgm_save_load))))

(event Custom|Spawn%20da%20thing
  (bind _returnvalue (Game|SpawnActorfromClass (Variables|Default|GetClass) (Transformation|GetWorldTransform (Variables|Default|GetSpawnLocation)) "DontSpawnIfColliding" "MultiplyWithRoot" 0 0))
  (Utilities|IsValid _returnvalue
    (:Is%20Valid
      (Development|PrintText "spawnd da thing"))
    (:Is%20Not%20Valid
      _))
  (Utilities|FlowControl|Delay 5.0)
  (CallFunction|SpawnDaThing))

(event EventBeginPlay
  (Utilities|FlowControl|Delay 1.0)
  (CallFunction|SpawnDaThing))

(event EventActivate
  (Actor|DestroyActor) ; if we aren't looping, destroy ourselves
)

(fn ConstructionScript)