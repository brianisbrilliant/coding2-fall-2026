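; AI controller for a security camera that raises an alarm when it senses a target.
; Perception updates branch first on stimulus tag, printing delayed, retriggerable text for footsteps, then on sense class display name for sight or hearing.
; Acquired sight plays a sound and sends every BP_DumDum to check the stimulus location; lost sight plays another sound.
; Hearing only prints debug text, and red/green material swaps are disconnected.
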(event OnTargetPerceptionUpdated(AIPerception)
  (params (Actor :type Actor%20Object%20Reference) (Stimulus :type AI%20Stimulus%20Structure))
  (bind (_age _expirationage _strength _stimuluslocation _receiverlocation _tag _bsuccessfullysensed) (Utilities|Struct|BreakAIStimulus Stimulus))
  (bind _returnvalue (Class|AIPerceptionSystem|GetSenseClassforStimulus Stimulus))
  (Development|PrintText (Utilities|Text|FormatText "Sensed: {actor} with {name} using tag: {tag}" Actor (Utilities|GetClassDisplayName _returnvalue) _tag))
  (switch name _tag ; ignore AI, doesn't work yet.
    (:Default
      (switch string (Utilities|GetClassDisplayName _returnvalue)
        (:AISense_Sight
          (CallFunction|HandleSight Actor _bsuccessfullysensed _stimuluslocation))
        (:AISense_Hearing
          (CallFunction|HandleHearing _tag))))
    (:Footstep
      (Utilities|FlowControl|RetriggerableDelay 5.0)
      (Development|PrintText "I hear footsteps" true true "(R=0.000000,G=0.660000,B=1.000000,A=1.000000)" 5.0))))

(event EventBeginPlay)

(event EventTick
  (params (DeltaSeconds :type Float%20%28single-precision%29)))

(fn ConstructionScript)

(fn HandleSight
  (params (Target :type Actor%20Object%20Reference) (Successfully%20Sensed :type Boolean) (Stimulus%20Location :type Vector))
  (bind _returnvalue (Transformation|GetActorLocation))
  (if Successfully%20Sensed
    (Development|PrintText "Acquired Target")
    (Audio|PlaySoundatLocation "/Engine/EditorSounds/Notifications/CompileFailed.CompileFailed" _returnvalue "0, 0, 0" 2.0 1.0 0.0 "/Game/Audio/Attenuation.Attenuation" 0 0 0)
    (bind _outactors (Actor|GetAllActorsOfClass "/Game/Blueprints/AI/BP_DumDum.BP_DumDum_C"))
    (for _array_element _outactors
      (Default|CheckOutSecurityAlarm _array_element Stimulus%20Location))
    (else
      (Development|PrintText "Lost Target")
      (Audio|PlaySoundatLocation "/Engine/EditorSounds/Notifications/CompileSuccess.CompileSuccess" _returnvalue "0, 0, 0" 2.0 1.0 0.0 "/Game/Audio/Attenuation.Attenuation" 0 0 0))))

(fn HandleHearing
  (params (tag :type Name))
  (switch name tag
    (:Default
      (Development|PrintText "I heard something"))))