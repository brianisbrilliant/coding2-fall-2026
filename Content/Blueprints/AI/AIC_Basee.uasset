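; AIC_Basee is an AI controller that turns perception updates into State Tree events, ignoring actors tagged AI.
; Sight stores the sensed actor and sends an Attacking event, while hearing, prediction and damage store the stimulus location and send Investigating.
; Losing sight starts a retriggerable delay that clears the sensed actor unless it is seen again.
; Every sight update is also forwarded to the possessed pawn.
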(event OnTargetPerceptionUpdated(AIPerception)
  (params (Actor :type Actor%20Object%20Reference) (Stimulus :type AI%20Stimulus%20Structure))
  (bind (_age _expirationage _strength _stimuluslocation _receiverlocation _tag _bsuccessfullysensed) (Utilities|Struct|BreakAIStimulus Stimulus))
  (if (not (Actor|ActorHasTag Actor "AI")) ; ignore AI
    (bind _returnvalue (Class|AIPerceptionSystem|GetSenseClassforStimulus Stimulus))
    (switch string (Utilities|GetClassDisplayName _returnvalue)
      (:AISense_Sight
        ;[0.15 0.15 0.15 0.5] Enter the Attacking state if we see a target (usually the player)
        (if _bsuccessfullysensed ; into view or out of view?
          (Variables|Default|SetCanSeeSensedActor true)
          (Variables|Default|SetSensedActor Actor)
          (Gameplay|StateTree|SendStateTreeEvent (Variables|Default|GetStateTreeAI) (Utilities|Struct|MakeStateTreeEvent "(TagName=\"Ai.Event.Attacking\")") :!class /Script/GameplayStateTreeModule.StateTreeComponent)
          (else
            (CallFunction|LoseSightDelay)))
        (Class|BPIPerceiver|HandleSight(Message) (Variables|Default|GetPossessed%20Pawn) Actor _bsuccessfullysensed _stimuluslocation))
      (:AISense_Hearing
        (Variables|Default|SetPoint%20of%20Interest _stimuluslocation :!label _label)
        (Gameplay|StateTree|SendStateTreeEvent (Variables|Default|GetStateTreeAI) (Utilities|Struct|MakeStateTreeEvent "(TagName=\"Ai.Event.Investigating\")") :!class /Script/GameplayStateTreeModule.StateTreeComponent))
      (:AISense_Prediction
        (goto _label))
      (:AISense_Damage
        (goto _label)))))

(event Custom|LoseSightDelay
  (Variables|Default|SetCanSeeSensedActor false)
  (Utilities|FlowControl|RetriggerableDelay 5.0) ; wait this long before the LAST time\nthat we lost sight of the player
  (if (not (Variables|Default|GetCanSeeSensedActor))
    (Variables|Default|SetSensedActor 0) ; Set sensed actor to NULL
  ))

(event EventPossess
  (params (PossessedPawn :type Pawn%20Object%20Reference))
  (Variables|Default|SetPossessed%20Pawn PossessedPawn)
  (Development|PrintText "AIC_Basee exists"))

(fn ConstructionScript)