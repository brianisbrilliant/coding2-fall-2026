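; Security camera actor that uses AI Perception to spot targets and raise an alarm.
; Perception updates route by stimulus tag and sense class name, sending sight to HandleSight and only printing for AI-tagged stimuli.
; Sight gained or lost swaps the mesh material and plays a sound; acquiring also sends every BP_DumDum the stimulus location via CheckOutSecurityAlarm.
; Forgetting a target applies a viewfinder material, with debug prints throughout.
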(event OnTargetPerceptionUpdated(AIPerception)
  (params (Actor :type Actor%20Object%20Reference) (Stimulus :type AI%20Stimulus%20Structure))
  (bind (_age _expirationage _strength _stimuluslocation _receiverlocation _tag _bsuccessfullysensed) (Utilities|Struct|BreakAIStimulus Stimulus))
  (bind _returnvalue (Class|AIPerceptionSystem|GetSenseClassforStimulus Stimulus))
  (Development|PrintText (Utilities|Text|FormatText "Sensed: {actor} with {name} using tag: {tag}" (Utilities|GetClassDisplayName _returnvalue) Actor _tag))
  (switch name _tag ; ignore AI, doesn't work yet.
    (:Default
      (switch string (Utilities|GetClassDisplayName _returnvalue)
        (:AISense_Sight
          (CallFunction|HandleSight Actor _bsuccessfullysensed _stimuluslocation))))
    (:AI
      (Development|PrintText "Hello AI buddy"))))

(event OnTargetPerceptionForgotten(AIPerception)
  (params (Actor :type Actor%20Object%20Reference))
  ;[0.15 0.15 0.15 0.5] How to handle forgetting about a target
  (Development|PrintText (Utilities|Text|FormatText "Forgot about {AAAAActor}" Actor))
  (Rendering|Material|SetMaterial (Variables|Default|GetStaticMesh) 0 "/Engine/EditorMeshes/Camera/MI_CineCam_ViewFinder.MI_CineCam_ViewFinder"))

(event OnTargetPerceptionInfoUpdated(AIPerception)
  (params (UpdateInfo :type Actor%20Perception%20Update%20Info%20Structure%20%28by%20ref%29))
  ;[0.15 0.15 0.15 0.5] How to handle forgetting about a target
)

(event EventBeginPlay)

(event Collision|EventActorBeginOverlap
  (params (OtherActor :type Actor%20Object%20Reference)))

(event EventTick
  (params (DeltaSeconds :type Float%20%28single-precision%29)))

(fn ConstructionScript)

(fn HandleSight
  (params (Target :type Actor%20Object%20Reference) (Successfully%20Sensed :type Boolean) (Stimulus%20Location :type Vector))
  (bind _returnvalue (Transformation|GetActorLocation))
  (bind _staticmesh (Variables|Default|GetStaticMesh))
  (if Successfully%20Sensed
    (Development|PrintText "Acquired Target")
    (Rendering|Material|SetMaterial _staticmesh 0 "/AnimationSharing/AnimSharingRed.AnimSharingRed")
    (Audio|PlaySoundatLocation "/Engine/EditorSounds/Notifications/CompileFailed.CompileFailed" _returnvalue "0, 0, 0" 2.0 1.0 0.0 "/Game/Audio/Attenuation.Attenuation" 0 0 0)
    (bind _outactors (Actor|GetAllActorsOfClass "/Game/Blueprints/AI/BP_DumDum.BP_DumDum_C"))
    (for _array_element _outactors
      (Default|CheckOutSecurityAlarm _array_element Stimulus%20Location))
    (else
      (Development|PrintText "Lost Target")
      (Rendering|Material|SetMaterial _staticmesh 0 "/AnimationSharing/AnimSharingGreen.AnimSharingGreen")
      (Audio|PlaySoundatLocation "/Engine/EditorSounds/Notifications/CompileSuccess.CompileSuccess" _returnvalue "0, 0, 0" 2.0 1.0 0.0 "/Game/Audio/Attenuation.Attenuation" 0 0 0))))