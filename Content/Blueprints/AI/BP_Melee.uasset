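; BP_Melee is a melee AI actor, judging by its name and folder, that takes damage and dies.
; AnyDamage reports a damage event at the instigator's pawn location, letting AI damage sensing locate the attacker.
; It then subtracts damage from Health, prints debug messages and destroys the actor once Health is no longer above zero.
; The file contains no attack logic, and its construction script is empty.
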(event Game|Damage|EventAnyDamage
  (params (Damage :type Float%20%28single-precision%29) (DamageType :type Damage%20Type%20Object%20Reference) (InstigatedBy :type Controller%20Object%20Reference) (DamageCauser :type Actor%20Object%20Reference))
  (Utilities|IsValid InstigatedBy
    (:Is%20Valid
      (Class|AISenseDamage|ReportDamageEvent self InstigatedBy Damage (Transformation|GetActorLocation (Pawn|GetControlledPawn InstigatedBy)) "0, 0, 0" "None"))
    (:Is%20Not%20Valid
      (Development|PrintText "health hit gave us life.")))
  (bind _output_get (Variables|Default|SetHealth (- (Variables|Default|GetHealth) Damage)))
  (Development|PrintText (Utilities|Text|FormatText "now i have {health} health." _output_get))
  (if (> _output_get 0.0) ; is health greater than zero?
    (Development|PrintText (Utilities|Text|FormatText "Ouch! Hurt for {amount} damage from {instigator}" Damage InstigatedBy))
    (else
      (Actor|DestroyActor) ; if not, destroy ourselves
    )))

(fn ConstructionScript)