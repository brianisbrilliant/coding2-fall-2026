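; BP_Ranged is an AI enemy, named as a ranged type, with health that damage reduces and med kits restore.
; On BeginPlay it caches its AIC_Basee controller.
; Damage is reported to AI perception at the instigator pawn's location and sent to the controller's StateTree as a TookDamage event.
; At zero health it is destroyed as a ragdoll placeholder, while healing clamps health to a 0–1 range.
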(event Custom|Get%20MedKit
  (params (HealthToAdd :type Float%20%28double-precision%29))
  (Variables|Default|SetHealth (Math|Float|Clamp(Float) (+ (Variables|Default|GetHealth) HealthToAdd))))

(event EventBeginPlay
  (bind _asaic_basee (Utilities|Casting|CastToAIC_Basee (Pawn|GetController)))
  (Variables|Default|SetAIC _asaic_basee) ; promote to variable
)

(event Game|Damage|EventAnyDamage
  (params (Damage :type Float%20%28single-precision%29) (DamageType :type Damage%20Type%20Object%20Reference) (InstigatedBy :type Controller%20Object%20Reference) (DamageCauser :type Actor%20Object%20Reference))
  (Class|AISenseDamage|ReportDamageEvent self InstigatedBy Damage (Transformation|GetActorLocation (Pawn|GetControlledPawn InstigatedBy)) "0, 0, 0" "None")
  (Gameplay|StateTree|SendStateTreeEvent (Variables|/Game/Blueprints/AI/AIC_Basee.AIC_Basee_C|GetStateTreeAI (Variables|Default|GetAIC)) (Utilities|Struct|MakeStateTreeEvent "(TagName=\"AI.Event.TookDamage\")") :!class /Script/GameplayStateTreeModule.StateTreeComponent)
  (bind _output_get (Variables|Default|SetHealth (- (Variables|Default|GetHealth) Damage)))
  (if (not (> _output_get 0.0)) ; Are we still alive?
    (Development|PrintText "We are DEAD")
    (Actor|DestroyActor) ; replace this with ragdoll
  ))

(fn ConstructionScript)