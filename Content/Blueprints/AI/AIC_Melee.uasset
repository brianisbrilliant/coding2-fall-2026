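; Melee AI controller that turns perception stimuli from actors not tagged AI into State Tree events.
; Sight sets the target actor and sends an Attacking event, while hearing and damage store the stimulus location as a point of interest and send Investigating.
; Losing sight starts a delay that clears the target unless the player is seen again before it ends.
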(event OnTargetPerceptionUpdated(AIPerception)
  (params (Actor :type Actor%20Object%20Reference) (Stimulus :type AI%20Stimulus%20Structure))
  (bind (_age _expirationage _strength _stimuluslocation _receiverlocation _tag _bsuccessfullysensed) (Utilities|Struct|BreakAIStimulus Stimulus))
  (if (not (Actor|ActorHasTag Actor "AI")) ; ignore actors with the AI tag
    (bind _returnvalue (Class|AIPerceptionSystem|GetSenseClassforStimulus Stimulus))
    (switch string (Utilities|GetClassDisplayName _returnvalue)
      (:AISense_Sight
        (CallFunction|HandleSight _bsuccessfullysensed Actor))
      (:AISense_Hearing
        (CallFunction|HandleSound _stimuluslocation))
      (:AISense_Damage
        (CallFunction|HandleDamage 0 _stimuluslocation)))))

(event Custom|LoseSightDelay
  (Variables|Default|SetCanSeePlayer false)
  (Utilities|FlowControl|Delay (Variables|Default|GetLoseSightDuration))
  (if (not (Variables|Default|GetCanSeePlayer))
    (Variables|Default|SetTarget%20Actor 0) ; Clear target actor
  ))

(event EventPossess
  (params (PossessedPawn :type Pawn%20Object%20Reference))
  (Variables|Default|SetPossessed%20Pawn PossessedPawn))

(fn ConstructionScript)

(fn HandleSight
  (params (Successfully%20Sensed :type Boolean) (Target%20Actor :type Actor%20Object%20Reference))
  (if Successfully%20Sensed
    (Variables|Default|SetCanSeePlayer true)
    (Variables|Default|SetTarget%20Actor Target%20Actor) ; assign target actor
    (Gameplay|StateTree|SendStateTreeEvent (Variables|Default|GetStateTreeAI) (Utilities|Struct|MakeStateTreeEvent "(TagName=\"AI.Event.Attacking\")") :!class /Script/GameplayStateTreeModule.StateTreeComponent)
    (else
      (CallFunction|LoseSightDelay) ; begin to forget about the player
    )))

(fn HandleSound
  (params (Location :type Vector))
  (Variables|Default|SetPointOfInterest Location)
  (Gameplay|StateTree|SendStateTreeEvent (Variables|Default|GetStateTreeAI) (Utilities|Struct|MakeStateTreeEvent "(TagName=\"AI.Event.Investigating\")") :!class /Script/GameplayStateTreeModule.StateTreeComponent))

(fn HandleDamage
  (params (Attacker :type Actor%20Object%20Reference) (PointOfInterest :type Vector))
  (Variables|Default|SetPointOfInterest PointOfInterest)
  (Gameplay|StateTree|SendStateTreeEvent (Variables|Default|GetStateTreeAI) (Utilities|Struct|MakeStateTreeEvent "(TagName=\"AI.Event.Investigating\")") :!class /Script/GameplayStateTreeModule.StateTreeComponent))