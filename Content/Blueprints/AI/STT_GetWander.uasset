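; StateTree task that picks a random navigable wander location for an AI character.
; On entering the state it queries the navmesh within Radius of Origin and stores the point in Location, without checking whether the query succeeded.
; A near-zero Origin counts as unset and is replaced by the character capsule's world location.
; The task only computes the point; it issues no movement and no finish call.
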(event EventLatentEnterState
  (params (Transition :type State%20Tree%20Transition%20Result%20Structure%20%28by%20ref%29))
  ;[0.15 0.15 0.15 0.5] If no origin is provided, move relative to AI's current position
  (if (Utilities|Operators|EqualEqual :A (Variables|Default|GetOrigin) :ErrorTolerance 0.1)
    (Variables|Default|SetOrigin (Transformation|GetWorldLocation (Variables|/Script/Engine.Character|GetCapsuleComponent (Variables|Context|GetCharacter)))))
  (bind _randomlocation (Class|NavigationSystemV1|GetRandomLocationinNavigableRadius (Variables|Default|GetOrigin) (Variables|Default|GetRadius) 0 0))
  (Variables|Output|SetLocation _randomlocation))