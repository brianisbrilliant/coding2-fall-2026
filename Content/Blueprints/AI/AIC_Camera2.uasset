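; AI controller for security cameras and turrets that routes perception updates to whichever device it possesses.
; On possess it caches the pawn as a BP_SecurityCamera or, failing that, a BP_Turret2.
; Perception updates skip actors tagged AI, print debug text, and forward sight stimuli to that pawn's HandleSight, with stimulus location passed only to the camera.
; A stimulus-tag check for AI only prints a message and is noted as not working yet.
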(event OnTargetPerceptionUpdated(AIPerception)
  (params (Actor :type Actor%20Object%20Reference) (Stimulus :type AI%20Stimulus%20Structure))
  (bind (_age _expirationage _strength _stimuluslocation _receiverlocation _tag _bsuccessfullysensed) (Utilities|Struct|BreakAIStimulus Stimulus))
  (if (not (Actor|ActorHasTag Actor "AI")) ; ignore AI Actors
    (bind _returnvalue (Class|AIPerceptionSystem|GetSenseClassforStimulus Stimulus))
    (Development|PrintText (Utilities|Text|FormatText "Sensed: {actor} with {name} using tag: {tag}" Actor (Utilities|GetClassDisplayName _returnvalue) _tag))
    (switch name _tag ; ignore AI, doesn't work yet.
      (:Default
        (switch string (Utilities|GetClassDisplayName _returnvalue)
          (:AISense_Sight
            (CallFunction|HandleSight Actor _bsuccessfullysensed _stimuluslocation))))
      (:AI
        (Development|PrintText "Hello AI buddy")))))

(event EventBeginPlay)

(event EventTick
  (params (DeltaSeconds :type Float%20%28single-precision%29)))

(event EventPossess
  (params (PossessedPawn :type Pawn%20Object%20Reference))
  (bind _asbp_security_camera (Utilities|Casting|CastToBP_SecurityCamera PossessedPawn)
    (:then
      (Variables|Default|SetAs%20BP%20Security%20Camera _asbp_security_camera))
    (:CastFailed
      (bind _asbp_turret_2 (Utilities|Casting|CastToBP_Turret2 PossessedPawn))
      (Variables|Default|SetAs%20BP%20Turret%202 _asbp_turret_2))))

(fn ConstructionScript)

(fn HandleSight
  (params (Target :type Actor%20Object%20Reference) (Successfully%20Sensed :type Boolean) (Stimulus%20Location :type Vector))
  (bind _as_bp_security_camera (Variables|Default|GetAs%20BP%20Security%20Camera)
    (:then
      (Default|HandleSight _as_bp_security_camera Target Successfully%20Sensed Stimulus%20Location))
    (:else
      (bind _as_bp_turret_2 (Variables|Default|GetAs%20BP%20Turret%202)
        (:then
          (Default|HandleSight _as_bp_turret_2 Target Successfully%20Sensed))
        (:else)))))