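; BP_Turret is an AI turret actor that turns toward the player and spawns bullets on a repeating timer.
; BeginPlay sets the tick interval, caches player character 0 and starts FireProjectile, which spawns BP_Bullet at SpawnPoint, then re-calls itself after a delay derived from FireRate.
; Tick snaps the rotation to face the player.
; The bullet impulse logic is disconnected, so the turret applies no launch velocity.
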(event Custom|Fire%20Projectile
  (bind _returnvalue (Game|SpawnActorfromClass "/Game/Blueprints/BP_Bullet.BP_Bullet_C" (Transformation|GetWorldTransform (Variables|Default|GetSpawnPoint)) "Undefined" "MultiplyWithRoot" 0 0))
  (Utilities|FlowControl|Delay (/ 6e+01 (Variables|Default|GetFireRate)))
  (CallFunction|FireProjectile))

(event EventBeginPlay
  (Actor|Tick|SetActorTickInterval (Variables|Default|GetTick%20Interval)) ; set fire rate
  (Variables|Default|Setplayer (Game|GetPlayerCharacter 0))
  (CallFunction|FireProjectile))

(event EventTick
  (params (DeltaSeconds :type Float%20%28single-precision%29))
  (Transformation|SetActorRotation (Math|Rotator|FindLookatRotation (Transformation|GetActorLocation) (Transformation|GetActorLocation (Variables|Default|Getplayer)))))

(fn ConstructionScript)