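; BP_ShopKeep is a shopkeeper actor that shows its inventory menu when the first-person character overlaps its sphere.
; BeginPlay creates a W_ChestMenuu widget bound to its BPCInventory component and prints the item count.
; Both begin and end overlap call OpenBarrel, which ignores its Reverse flag, adds the menu to the viewport, shows the player's inventory and prints debug text, including the first item's name.
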(event OnComponentBeginOverlap(Sphere)
  (params (OverlappedComponent :type Primitive%20Component%20Object%20Reference) (OtherActor :type Actor%20Object%20Reference) (OtherComp :type Primitive%20Component%20Object%20Reference) (OtherBodyIndex :type Integer) (bFromSweep :type Boolean) (SweepResult :type Hit%20Result%20Structure%20%28by%20ref%29))
  (bind _asbp_first_person_character (Utilities|Casting|CastToBP_FirstPersonCharacter OtherActor))
  (CallFunction|OpenBarrel false))

(event OnComponentEndOverlap(Sphere)
  (params (OverlappedComponent :type Primitive%20Component%20Object%20Reference) (OtherActor :type Actor%20Object%20Reference) (OtherComp :type Primitive%20Component%20Object%20Reference) (OtherBodyIndex :type Integer))
  (Utilities|Casting|CastToBP_FirstPersonCharacter OtherActor)
  (CallFunction|OpenBarrel true))

(event Custom|Open%20Barrel
  (params (Reverse :type Boolean))
  (Development|PrintText "greeting shopkeep")
  (UserInterface|Viewport|AddtoViewport (Variables|Default|Getmenuwidget) 0)
  (Default|ShowInventory (stale OnComponentBeginOverlap(Sphere) _asbp_first_person_character))
  (Development|PrintText (Utilities|Text|FormatText "First item in barrel is a {name}." (.Name (Utilities|Struct|BreakS_Item (Utilities|Array|Get(acopy) (Variables|/Game/Blueprints/BPC_Inventory.BPC_Inventory_C|Getinventory (Variables|Default|GetBPC_Inventory)))))) true true "(R=0.000000,G=0.660000,B=1.000000,A=1.000000)" 2e+01))

(event EventBeginPlay
  (bind _bpc_inventory (Variables|Default|GetBPC_Inventory))
  (bind _returnvalue (UserInterface|CreateWidget "/Game/Widgets/W_ChestMenuu.W_ChestMenuu_C" 0 _bpc_inventory))
  (Variables|Default|Setmenuwidget _returnvalue)
  (Development|PrintText (Utilities|Text|FormatText "There are {count} items" (Utilities|Array|Length (Variables|/Game/Blueprints/BPC_Inventory.BPC_Inventory_C|Getinventory _bpc_inventory)))))

(fn ConstructionScript)