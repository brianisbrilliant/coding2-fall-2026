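; Chest actor that opens when the first-person character enters its sphere trigger and closes when they leave.
; A shared openchest event plays or reverses the Open timeline, which lerps the hinge's roll to swing the lid.
; When opening finishes, it creates a W_ChestMenu widget with itself as the Chest and shows it.
; Leaving the sphere reverses the timeline and removes that menu; debug prints mark the stages.
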(event OnComponentBeginOverlap(Sphere)
  (params (OverlappedComponent :type Primitive%20Component%20Object%20Reference) (OtherActor :type Actor%20Object%20Reference) (OtherComp :type Primitive%20Component%20Object%20Reference) (OtherBodyIndex :type Integer) (bFromSweep :type Boolean) (SweepResult :type Hit%20Result%20Structure%20%28by%20ref%29))
  (Utilities|Casting|CastToBP_FirstPersonCharacter OtherActor)
  (Development|PrintText "Chest opening")
  (CallFunction|OpenChest false))

(event OnComponentEndOverlap(Sphere)
  (params (OverlappedComponent :type Primitive%20Component%20Object%20Reference) (OtherActor :type Actor%20Object%20Reference) (OtherComp :type Primitive%20Component%20Object%20Reference) (OtherBodyIndex :type Integer))
  (Utilities|Casting|CastToBP_FirstPersonCharacter OtherActor)
  (CallFunction|OpenChest true)
  (Development|PrintText "Hide GUI")
  (Widget|RemovefromParent (stale Custom|open%20chest _returnvalue)))

(event Custom|open%20chest
  (params (reverse :type Boolean))
  (if reverse
    (bind _newtrack_0 (Timeline|open Reverse)
      (:Update
        (Transformation|SetRelativeRotation (Variables|Default|Getrealhinge) (Math|Rotator|MakeRotator (Math|Float|Lerp 0.0 -7e+01 _newtrack_0) 0.0 0.0) false false))
      (:Finished
        (if (not reverse)
          (Development|PrintText "Show GUI")
          (bind _returnvalue (UserInterface|CreateWidget "/Game/Widgets/W_ChestMenu.W_ChestMenu_C" 0 0 self))
          (UserInterface|Viewport|AddtoViewport _returnvalue 0))))
    (else
      (Timeline|open Play))))

(event EventBeginPlay)

(event Collision|EventActorBeginOverlap
  (params (OtherActor :type Actor%20Object%20Reference)))

(event EventTick
  (params (DeltaSeconds :type Float%20%28single-precision%29)))

(fn ConstructionScript)