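; BP_Shopkeeper is a shop NPC that opens a trade menu when the player enters its sphere.
; BeginPlay creates W_ShopKeepMenu from its BPCInventory component.
; Sphere overlap shows that menu and the player's inventory and registers the shop inventory with GM_SaveLoad's LevelState; leaving removes only the shop menu.
; Activate restores BPCInventory from the saved InvActors map, looked up by the actor itself.
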(event OnComponentBeginOverlap(Sphere)
  (params (OverlappedComponent :type Primitive%20Component%20Object%20Reference) (OtherActor :type Actor%20Object%20Reference) (OtherComp :type Primitive%20Component%20Object%20Reference) (OtherBodyIndex :type Integer) (bFromSweep :type Boolean) (SweepResult :type Hit%20Result%20Structure%20%28by%20ref%29))
  (bind _asbp_first_person_character (Utilities|Casting|CastToBP_CustomChar OtherActor))
  (UserInterface|Viewport|AddtoViewport (stale EventBeginPlay _returnvalue) 0) ; show shop keep inventory
  (Default|ShowInventory _asbp_first_person_character) ; Show player inventory
  (bind _asgm_save_load (Utilities|Casting|CastToGM_SaveLoad (Game|GetGameMode)))
  (Default|AddInventory (Variables|/Game/Blueprints/SaveLoad/GM_SaveLoad.GM_SaveLoad_C|GetLevelState _asgm_save_load) (Variables|Default|GetBPC_Inventory)))

(event OnComponentEndOverlap(Sphere)
  (params (OverlappedComponent :type Primitive%20Component%20Object%20Reference) (OtherActor :type Actor%20Object%20Reference) (OtherComp :type Primitive%20Component%20Object%20Reference) (OtherBodyIndex :type Integer))
  (Utilities|Casting|CastToBP_CustomChar OtherActor)
  (Widget|RemovefromParent (stale EventBeginPlay _returnvalue)))

(event EventBeginPlay
  (bind _returnvalue (UserInterface|CreateWidget "/Game/UI/W_ShopKeepMenu.W_ShopKeepMenu_C" 0 (Variables|Default|GetBPC_Inventory))) ; set the menu inventory
)

(event EventActivate
  (bind _asgm_save_load (Utilities|Casting|CastToGM_SaveLoad (Game|GetGameMode)))
  (if (.ReturnValue (Utilities|Map|Find (Variables|/Game/Blueprints/SaveLoad/SG_LevelState.SG_LevelState_C|GetInvActors (Variables|/Game/Blueprints/SaveLoad/GM_SaveLoad.GM_SaveLoad_C|GetLevelState _asgm_save_load)) self))
    (Variables|Default|SetBPC_Inventory (.Value (Utilities|Map|Find (Variables|/Game/Blueprints/SaveLoad/SG_LevelState.SG_LevelState_C|GetInvActors (Variables|/Game/Blueprints/SaveLoad/GM_SaveLoad.GM_SaveLoad_C|GetLevelState _asgm_save_load)) self)))))

(fn ConstructionScript)