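; BP_Bullet is a projectile that damages BP_Enemy and BP_Melee actors it overlaps and destroys itself after a short lifetime.
; Its construction script copies the InitialSpeed variable into ProjectileMovement.
; Sphere overlaps subtract Health directly from BP_Enemy and destroy the bullet.
; BP_Melee instead receives ApplyDamage credited to the first player controller, and that branch leaves the bullet alive.
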(event OnComponentBeginOverlap(Sphere1)
  (params (OverlappedComponent :type Primitive%20Component%20Object%20Reference) (OtherActor :type Actor%20Object%20Reference) (OtherComp :type Primitive%20Component%20Object%20Reference) (OtherBodyIndex :type Integer) (bFromSweep :type Boolean) (SweepResult :type Hit%20Result%20Structure%20%28by%20ref%29))
  (bind _asbp_enemy (Utilities|Casting|CastToBP_Enemy OtherActor)
    (:then
      (Variables|/Game/Blueprints/Prep/Enemies/BP_Enemy.BP_Enemy_C|SetHealth _asbp_enemy (- (Variables|/Game/Blueprints/Prep/Enemies/BP_Enemy.BP_Enemy_C|GetHealth _asbp_enemy) 1e+01))
      (Actor|DestroyActor))
    (:CastFailed
      (bind _asbp_melee (Utilities|Casting|CastToBP_Melee OtherActor))
      (Game|Damage|ApplyDamage _asbp_melee 0.2 (Game|GetPlayerController 0) self))))

(event EventBeginPlay
  (Utilities|FlowControl|Delay 2.0)
  (Actor|DestroyActor))

(fn ConstructionScript
  (Variables|/Script/Engine.ProjectileMovementComponent|SetInitialSpeed (Variables|Default|GetProjectileMovement) (Variables|Default|GetInitial%20Speed)))