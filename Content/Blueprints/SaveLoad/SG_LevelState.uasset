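; SG_LevelState, in the SaveLoad folder, holds level state as lists of activated actors and inventories.
; AddActor and AddInventory append unique entries to their lists.
; ActivateActors replays activation by sending ActivateMessage to each valid stored actor, then prints a debug text.
; LoadInventories is an empty stub, and leftover map and nested-array nodes for inventory data never run.
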(event Custom|Add%20Actor
  (params (Actor :type Actor%20Object%20Reference%20%28by%20ref%29))
  (Utilities|Array|AddUnique (Variables|Default|GetActivatedActors) Actor))

(event Custom|Activate%20Actors
  (for _array_element (Variables|Default|GetActivatedActors)
    (Utilities|IsValid _array_element
      (:Is%20Valid
        (Class|BPIActivatable|Activate(Message) _array_element))))
  (Development|PrintText 0 "Activated all actors"))

(event Custom|Add%20Inventory
  (params (Inventory :type BPC%20Inventory%20Object%20Reference%20%28by%20ref%29))
  (Utilities|Array|AddUnique (Variables|Default|GetInventories) Inventory))

(event Custom|Load%20Inventories)