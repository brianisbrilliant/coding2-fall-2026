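; BP_Checkpoint is a checkpoint actor that saves the player's progress when the player character overlaps it.
; On BeginPlay it caches the GM_SaveLoad game mode.
; On overlap by BP_CustomChar it passes the belt and backpack inventories and the character's transform to the game mode's Save, then prints an activation message.
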(event EventBeginPlay
  (bind _asgm_save_load (Utilities|Casting|CastToGM_SaveLoad (Game|GetGameMode)))
  (Variables|Default|SetGame%20Mode _asgm_save_load))

(event Collision|EventActorBeginOverlap
  (params (OtherActor :type Actor%20Object%20Reference))
  (bind _asbp_first_person_character (Utilities|Casting|CastToBP_CustomChar OtherActor)) ; when player overlaps, call the save function on the game mode
  (Default|Save (Variables|Default|GetGame%20Mode) (Variables|/Game/Blueprints/BPC_Inventory.BPC_Inventory_C|GetEnumInv (Variables|/Game/Blueprints/BP_CustomChar.BP_CustomChar_C|GetBPC_Inv_Belt _asbp_first_person_character)) (Variables|/Game/Blueprints/BPC_Inventory.BPC_Inventory_C|GetEnumInv (Variables|/Game/Blueprints/BP_CustomChar.BP_CustomChar_C|GetBPC_Inv_Backpack _asbp_first_person_character)) (Transformation|GetActorTransform _asbp_first_person_character))
  (Development|PrintText "Checkpoint activated!"))

(fn ConstructionScript)