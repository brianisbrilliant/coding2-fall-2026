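; Game mode that saves and restores player inventory and per-level state through two SaveGame objects.
; SG_Player holds belt and backpack inventory in the base slot; SG_LevelState uses a slot suffixed with the level name.
; BeginPlay checks each slot, creating missing objects or calling the shared Load, which refills inventory, activates level actors and restores player transform and view.
; Save writes both slots; the delete functions clear slots and reopen the level.
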(event EventBeginPlay
  (Development|PrintText "Starting GM_ SaveLoad" true true "(R=1.000000,G=0.440535,B=0.000000,A=1.000000)" 5.0)
  (Utilities|FlowControl|Sequence
    (:then_0
      (bind _returnvalue (SaveGame|DoesSaveGameExist (Variables|Default|GetSlot%20Name)))
      (if _returnvalue
        (CallFunction|Load)
        (Development|PrintText "called load")
        (else
          (bind _returnvalue_2 (SaveGame|CreateSaveGameObject "/Game/Blueprints/SaveLoad/SG_Player.SG_Player_C"))
          (Variables|Default|SetPlayerSave _returnvalue_2)
          (Development|PrintText "created save game" :!label _label))))
    (:then_1
      ;[0.15 0.15 0.15 0.5] Load or create the level state save game.
      (bind _returnvalue_3 (Game|GetCurrentLevelName true))
      (bind _returnvalue_4 (SaveGame|DoesSaveGameExist (Utilities|String|Append (Variables|Default|GetSlot%20Name) "_" _returnvalue_3)))
      (if _returnvalue_4
        (CallFunction|Load)
        (else
          (bind _returnvalue_5 (SaveGame|CreateSaveGameObject "/Game/Blueprints/SaveLoad/SG_LevelState.SG_LevelState_C"))
          (Variables|Default|SetLevelState _returnvalue_5)
          (goto _label))))))

(fn ConstructionScript)

(fn Save
  (params (Belt :type Array%20of%20E_Item%20Enums :default "NewEnumerator0") (PlayerInv :type Array%20of%20E_Item%20Enums :default "NewEnumerator0") (Location :type Transform))
  (bind _playersave (Variables|Default|GetPlayerSave))
  (Utilities|FlowControl|Sequence
    (:then_0
      ;[0.15 0.15 0.15 0.5] Saving Player Stats
      (Variables|/Game/Blueprints/SaveLoad/SG_Player.SG_Player_C|SetBelt _playersave Belt)
      (Variables|/Game/Blueprints/SaveLoad/SG_Player.SG_Player_C|SetPlayerInv _playersave PlayerInv)
      (SaveGame|SaveGametoSlot (Variables|Default|GetPlayerSave) (Variables|Default|GetSlot%20Name)) ; save player stats to file
    )
    (:then_1
      ;[0.15 0.15 0.15 0.5] Saving Level State
      (Variables|/Game/Blueprints/SaveLoad/SG_LevelState.SG_LevelState_C|SetPlayerTransform (Variables|Default|GetLevelState) Location)
      (bind _returnvalue (Game|GetCurrentLevelName true))
      (SaveGame|SaveGametoSlot (Variables|Default|GetLevelState) (Utilities|String|Append (Variables|Default|GetSlot%20Name) "_" _returnvalue)) ; Save the level state to file
      (Development|PrintText "game saved to slot"))))

(fn Load
  (Utilities|FlowControl|Sequence
    (:then_0
      (bind _returnvalue (SaveGame|LoadGamefromSlot (Variables|Default|GetSlot%20Name))) ; load from file
      (bind _assg_player (Utilities|Casting|CastToSG_Player _returnvalue)) ; cast to specific SG_Player
      (Variables|Default|SetPlayerSave _assg_player) ; Store this as a variable
      (bind _asbp_first_person_character (Utilities|Casting|CastToBP_CustomChar (Game|GetPlayerCharacter 0)) ; get reference to player
        (:then
          (Default|SetEnumArray (Variables|/Game/Blueprints/BP_CustomChar.BP_CustomChar_C|GetBPC_Inv_Belt _asbp_first_person_character) (Variables|/Game/Blueprints/SaveLoad/SG_Player.SG_Player_C|GetBelt (Variables|Default|GetPlayerSave))) ; load in the belt that we saved
          (Default|SetEnumArray (Variables|/Game/Blueprints/BP_CustomChar.BP_CustomChar_C|GetBPC_Inv_Backpack _asbp_first_person_character) (Variables|/Game/Blueprints/SaveLoad/SG_Player.SG_Player_C|GetPlayerInv (Variables|Default|GetPlayerSave))) ; load in the player inventory that we saved
          (Development|PrintText "Inventory Updated"))
        (:CastFailed
          (Development|PrintText "cast failed"))))
    (:then_1
      (bind _returnvalue_2 (Game|GetCurrentLevelName true))
      (bind _returnvalue_3 (SaveGame|LoadGamefromSlot (Utilities|String|Append (Variables|Default|GetSlot%20Name) "_" _returnvalue_2)))
      (bind _assg_level_state (Utilities|Casting|CastToSG_LevelState _returnvalue_3))
      (bind _output_get (Variables|Default|SetLevelState _assg_level_state))
      (Default|ActivateActors _output_get)
      (bind _asbp_first_person_character_2 (Utilities|Casting|CastToBP_CustomChar (Game|GetPlayerCharacter 0))) ; get reference to player
      (Default|LoadTransform _asbp_first_person_character_2 (Variables|/Game/Blueprints/SaveLoad/SG_LevelState.SG_LevelState_C|GetPlayerTransform (Variables|Default|GetLevelState)) "0, 0, 0") ; Moving the player to the last saved position
      (Pawn|SetControlRotation (Game|GetPlayerController 0) (.Rotation (Math|Transform|BreakTransform (Variables|/Game/Blueprints/SaveLoad/SG_LevelState.SG_LevelState_C|GetPlayerTransform (Variables|Default|GetLevelState))))) ; loading the camera rotation\nthis should go in the Load Transform\nfunction on the first person character
    )))

(fn DeleteSave
  (SaveGame|DeleteGameinSlot (Variables|Default|GetSlot%20Name))
  (CallFunction|DeleteLevelSave))

(fn DeleteLevelSave
  (bind _returnvalue (Game|GetCurrentLevelName true))
  (SaveGame|DeleteGameinSlot (Utilities|String|Append (Variables|Default|GetSlot%20Name) "_" _returnvalue))
  (Game|OpenLevel(byName) (Utilities|String|StringToName _returnvalue)))