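; BP_Blaster is a blaster item that can be picked up, dropped and fired.
; Pickup turns off the collision box's collision and returns the item type, while Drop restores collision and physics and throws the item forward with an impulse.
; Use spawns a BP_Bullet at the spawn point and launches it along that point's forward vector with a velocity-change impulse scaled by BulletSpeed.
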(event EventUse
  (bind _bulletspawnpoint (Variables|Default|GetBulletSpawnPoint))
  (Development|PrintText "Zap!")
  (bind _returnvalue (Game|SpawnActorfromClass "/Game/Blueprints/BP_Bullet.BP_Bullet_C" (Transformation|GetWorldTransform _bulletspawnpoint) "Undefined" "MultiplyWithRoot" 0 3333.0 (Variables|Actor|GetInstigator)))
  (Class|PrimitiveComponent|AddVelocityChangeImpulseatLocation (Variables|/Game/Blueprints/BP_Bullet.BP_Bullet_C|GetSphere _returnvalue) (* (Math|Vector|GetForwardVector _bulletspawnpoint) (Variables|Default|GetBulletSpeed)) (Transformation|GetWorldLocation _bulletspawnpoint) "None"))

(event EventDrop
  (bind _collisionbox (Variables|Default|Getcollisionbox))
  (Collision|SetCollisionEnabled _collisionbox "QueryAndPhysics")
  (Physics|SetSimulatePhysics _collisionbox true)
  (Physics|AddImpulse _collisionbox (* (Math|Vector|GetForwardVector _collisionbox) 1e+03) "None" true))

(fn ConstructionScript)

(fn Pickup
  (params (Owner :type BPC%20Interact%20Object%20Reference%20%28by%20ref%29))
  (Collision|SetCollisionEnabled (Variables|Default|Getcollisionbox) "NoCollision")
  (return (Variables|Default|GetItemType)))