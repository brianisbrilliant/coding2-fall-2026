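; GM_SaveLoad is a Game Mode that saves and restores the player's belt, backpack inventory and last position through an SG_Player save object.
; On BeginPlay it loads the named slot, or creates a fresh save object if none exists, then pushes saved data into the first-person character's inventory components and moves its capsule unless the saved location is zero.
; SavePlayer writes the supplied data to the slot and prints the result.
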(event Custom|LoadPlayer
  ;[0.15 0.15 0.15 0.5] File Management
  (bind _returnvalue (SaveGame|DoesSaveGameExist (Variables|Default|GetSlot%20Name)))
  (if _returnvalue
    (bind _returnvalue_2 (SaveGame|LoadGamefromSlot (Variables|Default|GetSlot%20Name)))
    (bind _assg_player (Utilities|Casting|CastToSG_Player _returnvalue_2))
    (Variables|Default|SetPlayerSave _assg_player) ; we have linked the Game Mode's \nplayerSave with the 'saved-to-file'\nplayer save.
    (bind _asbp_first_person_character (Utilities|Casting|CastToBP_FirstPersonCharacter (Game|GetPlayerCharacter 0)))
    (Default|SetInventory (Variables|/Game/FirstPerson/Blueprints/BP_FirstPersonCharacter.BP_FirstPersonCharacter_C|GetBPC_Inv_Belt _asbp_first_person_character) (Variables|/Game/Blueprints/SavingLoading/SG_Player.SG_Player_C|GetBelt (Variables|Default|GetPlayerSave))) ; load the belt
    (Default|SetInventory (Variables|/Game/FirstPerson/Blueprints/BP_FirstPersonCharacter.BP_FirstPersonCharacter_C|GetBPC_Inv_Backpack _asbp_first_person_character) (Variables|/Game/Blueprints/SavingLoading/SG_Player.SG_Player_C|GetInventory (Variables|Default|GetPlayerSave))) ; load the player inventory
    ;[0.15 0.15 0.15 0.5] is there save data for the location?
    (if (not (Class|KismetMathLibrary|EqualExactlyVectorVector (.Location (Math|Transform|BreakTransform (Variables|/Game/Blueprints/SavingLoading/SG_Player.SG_Player_C|GetLast%20Position (Variables|Default|GetPlayerSave)))) "0, 0, 0")) ; Is the last transform set to 0,0,0?\nif so, do nothing.
      (Transformation|SetWorldTransform (Variables|/Script/Engine.Character|GetCapsuleComponent _asbp_first_person_character) (Variables|/Game/Blueprints/SavingLoading/SG_Player.SG_Player_C|GetLast%20Position (Variables|Default|GetPlayerSave)) false false))
    (else
      (bind _returnvalue_3 (SaveGame|CreateSaveGameObject "/Game/Blueprints/SavingLoading/SG_Player.SG_Player_C"))
      (Variables|Default|SetPlayerSave _returnvalue_3))))

(event Custom|SavePlayer
  (params (Belt :type Array%20of%20E_Item%20Enums :default "NewEnumerator0") (Inventory :type Array%20of%20E_Item%20Enums :default "NewEnumerator0") (InputPin :type Transform))
  (bind _playersave (Variables|Default|GetPlayerSave))
  (Variables|/Game/Blueprints/SavingLoading/SG_Player.SG_Player_C|SetBelt _playersave Belt)
  (Variables|/Game/Blueprints/SavingLoading/SG_Player.SG_Player_C|SetInventory _playersave Inventory)
  (Variables|/Game/Blueprints/SavingLoading/SG_Player.SG_Player_C|SetLast%20Position _playersave InputPin)
  (bind _returnvalue (SaveGame|SaveGametoSlot (Variables|Default|GetPlayerSave) (Variables|Default|GetSlot%20Name)))
  (if _returnvalue
    (Development|PrintText "Game saved to slot" true true "(R=0.080009,G=1.000000,B=0.000000,A=1.000000)")
    (else
      (Development|PrintText "Could not save game to slot" true true "(R=1.000000,G=0.000000,B=0.050000,A=1.000000)"))))

(event EventBeginPlay
  (Development|PrintText "GM_SaveLoad is running" true true "(R=1.000000,G=0.857322,B=0.177829,A=1.000000)" 5.0)
  (CallFunction|LoadPlayer))

(fn ConstructionScript)