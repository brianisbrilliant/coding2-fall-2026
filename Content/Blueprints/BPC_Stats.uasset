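; BPC_Stats is a stats component that tracks stamina and shows it on screen through a W_Stats widget created at BeginPlay.
; Tick regenerates stamina by a fixed, frame-rate-dependent step until full.
; SetStamina applies a clamped delta, rebuilds the Stats struct, updates the widget text and returns whether any meaningful stamina remains.
; GetStamina is an empty stub.
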(event EventBeginPlay
  (bind _returnvalue (UserInterface|CreateWidget "/Game/UI/W_Stats.W_Stats_C"))
  (bind _output_get (Variables|Default|SetStats%20Widget _returnvalue))
  (UserInterface|Viewport|AddtoViewport _output_get 0))

(event EventTick
  (params (DeltaSeconds :type Float%20%28single-precision%29))
  ;[0.15 0.15 0.15 0.5] Recharge Stamina if below 100
  (if (< (.stamina (Variables|Default|GetStats)) 1e+02)
    (CallFunction|SetStamina 1.0)))

(fn GetStamina)

(fn SetStamina
  (params (by%20amount :type Float%20%28double-precision%29))
  (bind _output_get (Variables|Default|SetStats (Utilities|Struct|MakeS_Stats 0.0 0.0 (Math|Float|Clamp(Float) (+ (.stamina (Variables|Default|GetStats)) by%20amount) 0.0 1e+02) "0.000000,0.000000,0.000000|0.000000,0.000000,-0.000000|1.000000,1.000000,1.000000" 0.0 0.0))) ; update our stamina.
  (Rendering|Components|TextRender|SetText (Variables|/Game/UI/W_Stats.W_Stats_C|GetTxt_StaminaAmount (Variables|Default|GetStats%20Widget)) (Utilities|Text|ToText(Float) (.stamina _output_get) "HalfToEven")) ; Update Widget
  (if (> (.stamina _output_get) 0.5)
    (return true)
    (else
      (return false))))