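; BP_Key is a carried key item that opens doors and can point to the nearest one.
; Pickup stores the owner and disables collision, while Drop restores physics and throws the key forward.
; Use line-traces ahead for a BP_Door, has the owner drop the key, then opens the door and destroys itself.
; AltUse draws a debug line to the closest valid door from an array cached at BeginPlay.
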(event EventAltUse
  (bind (_closestactor _isempty) (CallFunction|GetClosest (Variables|Default|GetDoors) self))
  (if (not _isempty)
    (Rendering|Debug|DrawDebugLine (Transformation|GetActorLocation) (Transformation|GetActorLocation _closestactor) "(R=1.000000,G=0.161384,B=0.634166,A=1.000000)" 4.0 5.0)))

(event EventUse
  (bind _box1 (Variables|Default|GetBox1))
  (bind _returnvalue (Transformation|GetWorldLocation _box1))
  (bind (_outhit _returnvalue_2) (Collision|LineTraceByChannel _returnvalue (+ _returnvalue (* (Math|Vector|GetForwardVector _box1) 4e+02)) "TraceTypeQuery1" false 0 "ForDuration"))
  (if _returnvalue_2 ; did we hit something?
    (bind _asbp_door (Utilities|Casting|CastToBP_Door (.HitActor (Collision|BreakHitResult _outhit)))) ; did we hit a door?
    (Default|TrytoDrop (Variables|Default|GetOwner_0))
    (Utilities|FlowControl|Delay 0.2)
    (Default|OpenDoor _asbp_door) ; open the door
    (Actor|DestroyActor self) ; destroy key
  ))

(event EventDrop
  (bind _box1 (Variables|Default|GetBox1))
  (Collision|SetCollisionEnabled _box1 "QueryAndPhysics")
  (Physics|SetSimulatePhysics _box1 true)
  (Physics|AddImpulse _box1 (* (Math|Vector|GetForwardVector _box1) 1e+03) "None" true))

(event EventBeginPlay
  (bind _outactors (Actor|GetAllActorsOfClass "/Game/Blueprints/BP_Door.BP_Door_C"))
  (Variables|Default|SetDoors _outactors) ; Promote to Variable
)

(fn ConstructionScript)

(fn GetClosest
  (params (ArrayOfActors :type Array%20of%20Actor%20Object%20References) (Origin :type Actor%20Object%20Reference))
  (bind _returnvalue (Utilities|Array|IsEmpty ArrayOfActors))
  (if _returnvalue
    (return 0 _returnvalue)
    (else
      (for _array_element ArrayOfActors
        (Utilities|IsValid _array_element ; Check for missing doors in the \nDoors array
          (:Is%20Valid
            (if (<= (Transformation|GetDistanceTo _array_element Origin) (LocalVariables|GetLowestScore))
              (LocalVariables|SetLowestScore (Transformation|GetDistanceTo _array_element Origin))
              (LocalVariables|SetClosestSoFar _array_element)))))
      (return (LocalVariables|GetClosestSoFar) _returnvalue))))

(fn Pickup
  (params (Owner :type BPC%20Interact%20Object%20Reference%20%28by%20ref%29))
  (Variables|Default|SetOwner_0 Owner)
  (Collision|SetCollisionEnabled (Variables|Default|GetBox1) "NoCollision") ; Stop the key from pushing the player off the map
  (return (Variables|Default|GetItemType)))